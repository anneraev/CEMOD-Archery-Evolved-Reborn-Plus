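; Thrown projectile weapon Blueprint that applies power-charge effects to the projectile it launches.
; SetCombo edits the projectile's combo structure in two passes: damage type, then effects.
; The damage pass adds hit and block modifiers per PowerChargeMultipliers entry while combat is in a specific substate.
; The effects pass maps charge to flinch, push or knockdown knockback; its former Accuracy_40 perk check is disconnected.
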(event EventSetCombo
  (params (BaseCombat :type Base%20BP%20Combat%20Object%20Reference) (BaseProjectile :type BP%20Base%20Projectile%20Object%20Reference))
  (CallFunction|HandlePowerChargeforDamageType BaseCombat BaseProjectile)
  (CallFunction|HandlePowerChargeEffects BaseCombat BaseProjectile))

(fn HandlePowerChargeforDamageType
  (params (Combat :type Base%20BP%20Combat%20Object%20Reference) (Projectile :type BP%20Base%20Projectile%20Object%20Reference))
  (bind _returnvalue (|GetPowerChargeMod2))
  (Default|GetComboCurrent Combat)
  (LocalVariables|SetLocal%20Combo (LocalVariables|GetLocal%20Combo))
  (for _array_element (Variables|PowerCharge|GetPower%20Charge%20Multipliers)
    (if (Default|InSubstate (LocalVariables|GetLocal%20Combat) "NewEnumerator25")
      (Utilities|Array|Add (.DamageModifiers (Utilities|Struct|BreakSTR_ComboStep (LocalVariables|GetLocal%20Combo))) (Utilities|Struct|MakeSTR_ComboStepDamageMod _array_element _returnvalue _returnvalue))))
  (Variables|/Game/Items/Weapons/BP_BaseProjectile.BP_BaseProjectile_C|SetComboStructure Projectile (LocalVariables|GetLocal%20Combo))
  (return))

(fn HandlePowerChargeEffects
  (params (Combat :type Base%20BP%20Combat%20Object%20Reference) (Projectile :type BP%20Base%20Projectile%20Object%20Reference))
  (bind _output_get (LocalVariables|SetLocal%20Combat Combat))
  (Utilities|IsValid _output_get
    (:Is%20Valid
      (bind _output_get_2 (LocalVariables|SetLocal%20Projectile Projectile))
      (Utilities|IsValid _output_get_2
        (:Is%20Valid
          (bind _combocurrent (Default|GetComboCurrent (LocalVariables|GetLocal%20Combat)))
          (LocalVariables|SetLocal%20Combo _combocurrent)
          (bind _structout (Utilities|Struct|SetmembersinSTR_ComboStep (Variables|/Game/Items/Weapons/BP_BaseProjectile.BP_BaseProjectile_C|GetComboStructure (LocalVariables|GetLocal%20Projectile)) (Utilities|Select :Index (Math|Float|Floor (Math|Float|MapRangeUnclamped (Default|GetPowerChargeModifier (LocalVariables|GetLocal%20Combat)) 0.0 1.0 0.0 2.0)) :Option%200 "/Game/Systems/Combat/DamageTypes/BP_Knockback_FlinchAway_Accuracy40_Perk.BP_Knockback_FlinchAway_Accuracy40_Perk_C" :Option%201 "/Game/Systems/Combat/DamageTypes/BP_Knockback_PushAway_Accuracy40_Perk.BP_Knockback_PushAway_Accuracy40_Perk_C" :Option%202 "/Game/Systems/Combat/DamageTypes/BP_Knockback_Knockdown_Accuracy40_Perk.BP_Knockback_Knockdown_Accuracy40_Perk_C")))
          (Variables|/Game/Items/Weapons/BP_BaseProjectile.BP_BaseProjectile_C|SetComboStructure (LocalVariables|GetLocal%20Projectile) _structout)
          (return))
        (:Is%20Not%20Valid
          _)))
    (:Is%20Not%20Valid
      _))
  (return))