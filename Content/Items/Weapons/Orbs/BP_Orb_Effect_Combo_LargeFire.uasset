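; Large fire combo effect for orb weapons that deals periodic area damage around itself.
; On the server, a ticker fires every half second while PvP is allowed or the instigator is valid, and is removed on EndPlay.
; Each tick applies full armor-ignoring health damage, then explosive radial damage scaled inversely to the fade delay.
; The damage radius is derived at construction as three quarters of the Sphere radius.
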(event Custom|DoDamage
  (params (DeltaTime :type Float%20%28single-precision%29))
  (bind _returnvalue (Transformation|GetActorLocation))
  (bind _self self)
  (bind _instigator (Variables|Default|GetInstigator))
  (bind _damageradius (Variables|Default|GetDamageRadius))
  (bind _returnvalue_2 (Pawn|GetController _instigator))
  (bind _asconan_game_state (Utilities|Casting|CastToConanGameState (Game|GetGameState)))
  (if (or (Class|ConanGameState|IsPVPAllowed _asconan_game_state) (Utilities|IsValid (Variables|Default|GetInstigator)))
    (|ApplyRadialDamageAsync 8.0 _returnvalue _damageradius "/Game/Systems/Progression/DmgTypeHealth_IgnoreArmor_BP.DmgTypeHealth_IgnoreArmor_BP_C" 0 _self _returnvalue_2 true "ECC_Visibility"
      (:then
        (|ApplyRadialDamageAsync (/ 1e+03 (Variables|Default|GetDelayUntilFadeEffects)) _returnvalue _damageradius "/Game/Systems/Combat/Dmg_Explosive.Dmg_Explosive_C" 0 _self _returnvalue_2 false "ECC_Visibility")))))

(event EventBeginPlay
  (|CallParentFunction)
  (if (Networking|IsServer)
    (bind _returnvalue (Class|FuncomGenericLibrary|AddTickerDelegate (delegate Custom|DoDamage) 0.5))
    (Variables|Default|SetDoDamageHandle _returnvalue)))

(event EventEndPlay
  (params (EndPlayReason :type EEndPlayReason%20Enum :default "Destroyed"))
  (Class|FuncomGenericLibrary|RemoveTickerDelegateHandle (Variables|Default|GetDoDamageHandle))
  (|CallParentFunction EndPlayReason))

(fn ConstructionScript
  (|CallParentFunction)
  (Variables|Default|SetDamageRadius (* (Variables|/Script/Engine.SphereComponent|GetSphereRadius (Variables|Default|GetSphere)) 0.75)))