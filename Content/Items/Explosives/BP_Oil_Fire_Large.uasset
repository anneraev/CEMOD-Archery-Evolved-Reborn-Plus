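; Large oil fire area hazard that deals periodic armor-ignoring radial damage while burning.
; The server runs the damage ticker, gated by PvP being allowed or a valid instigator, and line-traces random box points down for small fire locations.
; RepNotifies spawn emitters there, scaled down with distance from center, and remove them when fires deactivate.
; Outside dedicated servers, timelines drive dynamic decal materials for ignition and fade-out, plus light intensity on ignition.
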(event Custom|CreateDamageOverTime
  ;[1 1 1] DamageOverTime
  (if (Networking|IsServer)
    (bind _returnvalue (Class|FuncomGenericLibrary|AddTickerDelegate (delegate Custom|DoDamage) 0.5))
    (Variables|Default|SetDoDamageHandle _returnvalue)))

(event Custom|DestroyLittleFires
  (Variables|Replication|SetFiresAreActive false))

(event Custom|StartOilFire
  ;[1 1 1] OilFireSytems
  (bind (_direction _oil_mask_radius _flame_mask_radius _flame_density _light_intensity) (Timeline|DecalActivation PlayFromStart)
    (:Update
      (CallFunction|SetParametersOilFireMaterials (Utilities|Array|MakeArray "Oil Mask Radius" "Flame Mask Radius" "Flame Density") (Utilities|Array|MakeArray _oil_mask_radius _flame_mask_radius _flame_density))
      (Rendering|Components|Light|SetIntensity (Variables|Default|GetExplosion%20Light) (* _light_intensity 5e+03)))))

(event Custom|SpawnLittleFires
  (bind _boxforrandompoints (Variables|Default|GetBoxForRandomPoints))
  (bind _returnvalue (Class|FuncomGenericLibrary|GetRandomPointinBox _boxforrandompoints))
  (if (Networking|IsServer)
    (for _index (range 1 (Variables|Default|GetMaxLittleFires))
      (bind _outhit (Collision|LineTraceByChannel _returnvalue (- _returnvalue "0, 0,1000.000000") "TraceTypeQuery1" false 0 "None" true "(R=1.000000,G=0.000000,B=0.000000,A=1.000000)" "(R=0.000000,G=1.000000,B=0.000000,A=1.000000)" 15.0))
      (Utilities|Array|AddUnique (Variables|Default|GetLittleFireLocations) (.Location (Collision|BreakHitResult _outhit))))
    (Variables|Replication|SetFiresAreActive true)))

(event Custom|DoDamage
  (params (DeltaTime :type Float%20%28single-precision%29))
  (bind _returnvalue (Transformation|GetActorLocation))
  (bind _self self)
  (bind _instigator (Variables|Default|GetInstigator))
  (bind _damageradius (Variables|Default|GetDamageRadius))
  (bind _returnvalue_2 (Pawn|GetController _instigator))
  ;[1 1 1] DamageOverTime
  (bind _asconan_game_state (Utilities|Casting|CastToConanGameState (Game|GetGameState)))
  (if (or (Class|ConanGameState|IsPVPAllowed _asconan_game_state) (Utilities|IsValid (Variables|Default|GetInstigator)))
    (|ApplyRadialDamageAsync 12.0 _returnvalue _damageradius "/Game/Systems/Progression/DmgTypeHealth_IgnoreArmor_BP.DmgTypeHealth_IgnoreArmor_BP_C" 0 _self _returnvalue_2 false "ECC_Visibility"
      (:then
        (|ApplyRadialDamageAsync (/ 12.0 (Variables|Default|GetDelayUntilFadeEffects)) _returnvalue _damageradius "/Game/Systems/Progression/DmgTypeHealth_IgnoreArmor_BP.DmgTypeHealth_IgnoreArmor_BP_C" 0 _self _returnvalue_2 false "ECC_Visibility")))))

(event EventBeginPlay
  (|CallParentFunction)
  (if (Networking|IsServer)
    (CallFunction|CreateDamageOverTime)
    (CallFunction|SpawnLittleFires)))

(event EventMulticastStopEffect
  (params (Actor :type Actor%20Object%20Reference))
  ;[1 1 1] OilFireSytems
  (if (not (Networking|IsDedicatedServer))
    (bind (_direction _oil_decal_erosion _flame_density) (Timeline|DecalDe-Activation Play)
      (:Update
        (CallFunction|SetParametersOilFireMaterials (Utilities|Array|MakeArray "Erosion Softness" "Flame Density") (Utilities|Array|MakeArray _oil_decal_erosion _flame_density))))))

(event EventEndPlay
  (params (EndPlayReason :type EEndPlayReason%20Enum :default "Destroyed"))
  ;[1 1 1] End Play
  (Class|FuncomGenericLibrary|RemoveTickerDelegateHandle (Variables|Default|GetDoDamageHandle))
  (CallFunction|DestroyLittleFires)
  (|CallParentFunction EndPlayReason))

(event EventTurnonEffects
  (if (not (Networking|IsDedicatedServer))
    (Utilities|FlowControl|Sequence
      (:then_0
        (CallFunction|CreateDynamicOilFireMaterials))
      (:then_1
        (CallFunction|StartOilFire)))))

(fn ConstructionScript
  (|CallParentFunction)
  (Variables|Default|SetDamageRadius (* (Variables|/Script/Engine.SphereComponent|GetSphereRadius (Variables|Default|GetSphere)) 1.0)))

(fn CreateDynamicOilFireMaterials
  (for _array_element (Actor|GetComponentsbyTag "/Script/Engine.DecalComponent" "OilFireDecal")
    (Transformation|SetWorldScale3D _array_element (* (Transformation|GetWorldScale _array_element) 1.65))
    (bind _returnvalue (Rendering|Material|CreateDynamicMaterialInstance _array_element :!class /Script/Engine.DecalComponent))
    (Rendering|Material|SetScalarParameterValue _returnvalue "Erosion Amount" 0.0 :!class /Script/Engine.MaterialInstanceDynamic)
    (Rendering|Material|SetScalarParameterValue _returnvalue "Fade" 0.0 :!class /Script/Engine.MaterialInstanceDynamic)
    (Utilities|Array|AddUnique (Variables|Default|GetOilFireDynamicMaterials) _returnvalue)))

(fn OnRepFiresAreActive
  (bind _spawnedlittlefires (Variables|Default|GetSpawnedLittleFires))
  (if (not (Networking|IsDedicatedServer))
    (if (Variables|Replication|GetFiresAreActive)
      (for _array_element (Variables|Default|GetLittleFireLocations)
        (bind _returnvalue (Effects|SpawnEmitteratLocation "/Game/VFX/Particle_Systems/Fire/P_OilFireSolo_01.P_OilFireSolo_01" _array_element))
        (Transformation|SetWorldScale3D _returnvalue (+ (Transformation|GetWorldScale _returnvalue) (Math|Vector|MakeVector (Math|Float|MapRangeClamped (Math|Vector|VectorLength (- (Transformation|GetWorldLocation (Variables|Default|GetDefaultSceneRoot)) (Transformation|GetWorldLocation _returnvalue))) 0.0 8e+02 1.75 -0.9) (Math|Float|MapRangeClamped (Math|Vector|VectorLength (- (Transformation|GetWorldLocation (Variables|Default|GetDefaultSceneRoot)) (Transformation|GetWorldLocation _returnvalue))) 0.0 8e+02 1.75 -0.9) (Math|Float|MapRangeClamped (Math|Vector|VectorLength (- (Transformation|GetWorldLocation (Variables|Default|GetDefaultSceneRoot)) (Transformation|GetWorldLocation _returnvalue))) 0.0 8e+02 1.75 -0.9))))
        (Utilities|Array|AddUnique (Variables|Default|GetSpawnedLittleFires) _returnvalue))
      (else
        (for _array_element_2 _spawnedlittlefires
          (Components|Activation|Deactivate _array_element_2))
        (for _array_element_3 _spawnedlittlefires
          (Components|DestroyComponent _array_element_3))))))

(fn OnRepLittleFireLocations
  (for _array_element (Variables|Default|GetLittleFireLocations)
    (bind _returnvalue (Effects|SpawnEmitteratLocation "/Game/VFX/Particle_Systems/Fire/P_OilFireSolo_01.P_OilFireSolo_01" _array_element))
    (Transformation|SetWorldScale3D _returnvalue (+ (Transformation|GetWorldScale _returnvalue) (Math|Vector|MakeVector (Math|Float|MapRangeClamped (Math|Vector|VectorLength (- (Transformation|GetWorldLocation (Variables|Default|GetDefaultSceneRoot)) (Transformation|GetWorldLocation _returnvalue))) 0.0 8e+02 1.75 -0.9) (Math|Float|MapRangeClamped (Math|Vector|VectorLength (- (Transformation|GetWorldLocation (Variables|Default|GetDefaultSceneRoot)) (Transformation|GetWorldLocation _returnvalue))) 0.0 8e+02 1.75 -0.9) (Math|Float|MapRangeClamped (Math|Vector|VectorLength (- (Transformation|GetWorldLocation (Variables|Default|GetDefaultSceneRoot)) (Transformation|GetWorldLocation _returnvalue))) 0.0 8e+02 1.75 -0.9))))
    (Utilities|Array|AddUnique (Variables|Default|GetSpawnedLittleFires) _returnvalue)))

(fn SetParametersOilFireMaterials
  (params (ParameterNames :type Array%20of%20Names) (ParameterValues :type Array%20of%20Floats%20%28single-precision%29))
  (bind _returnvalue (Utilities|Array|Length ParameterValues))
  (if (== (Utilities|Array|Length ParameterNames) _returnvalue)
    (for _array_element (Variables|Default|GetOilFireDynamicMaterials)
      (for _index (range 0 (- _returnvalue 1))
        (Rendering|Material|SetScalarParameterValue _array_element (Utilities|Array|Get(acopy) ParameterNames _index) (Utilities|Array|Get(acopy) ParameterValues _index) :!class /Script/Engine.MaterialInstanceDynamic)))))