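; Elite demonology follower NPC that hunts the player who summoned it, then removes itself.
; On the server, non-thrall versions resolve the summoner UID, add massive provoke hate and bind once to that player's death and target-loss events.
; Either event stops movement, then destroys the actor after a delay, with a taunt and portal effect off dedicated servers.
; A replicated Hidden flag toggles mesh, particles and nameplate; unhiding plays a taunt.
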(event Custom|AddPlayerHate
  (params (PlayerToHate :type Conan%20Character%20Object%20Reference))
  (bind _bptargetdistributioncomponent (Variables|Default|GetBPTargetDistributionComponent))
  (Variables|Default|SetPlayerToHate PlayerToHate)
  (Utilities|FlowControl|Sequence
    (:then_0
      (Default|AddtoHatelist _bptargetdistributioncomponent (Utilities|Struct|MakeTargetWrapper (Variables|Default|GetPlayerToHate) -1))
      (Class|TargetDistributionComponent|AddHatetoTarget _bptargetdistributioncomponent (Utilities|Struct|MakeTargetWrapper (Variables|Default|GetPlayerToHate) -1) "ProvokeHate" 1e+04)
      (Development|PrintString (Utilities|String|Append "ADDED HATE FOR: " (Class|ConanCharacter|GetCharacterName (Variables|Default|GetPlayerToHate))) true true "(R=0.000000,G=0.660000,B=1.000000,A=1.000000)" 2e+01))
    (:then_1
      (Utilities|FlowControl|DoOnce false
        (:Completed
          (CallFunction|BindHateEvents))))))

(event Custom|PlayerDied
  (params (Character :type Conan%20Character%20Object%20Reference) (Killer :type Conan%20Character%20Object%20Reference))
  ;[1 0 0] REMOVE PRINT STR!!!
  (Development|PrintString "Player Died" true true "(R=0.000000,G=0.660000,B=1.000000,A=1.000000)" 2e+01)
  (Pawn|Components|CharacterMovement|DisableMovement (Variables|Character|GetCharacterMovement))
  (if (not (Networking|IsDedicatedServer))
    (bind _returnvalue (Animation|PlayAnimMontage "/Game/Characters/NPCs/Demonolgy_follower/Animations/AM_demonologyfollower_combat_taunt.AM_demonologyfollower_combat_taunt" 1.0 "None"))
    (Utilities|FlowControl|Delay _returnvalue)
    (Effects|SpawnEmitteratLocation "/Game/Sorcery/Craftingstations/Chalk_Circle/Effects/P_chalk_circle_portal_Interrupt.P_chalk_circle_portal_Interrupt" (Transformation|GetActorLocation))
    (else
      (Utilities|FlowControl|Delay 3.0)))
  (Actor|DestroyActor))

(event Custom|TargetLost
  (params (Target :type Target%20Wrapper%20Structure%20%28by%20ref%29))
  ;[1 0 0] REMOVE PRINT STR!!!
  (Development|PrintString "target lost" true true "(R=0.000000,G=0.660000,B=1.000000,A=1.000000)" 2e+01)
  (if (== (Utilities|ToObject(Interface) (.RawTarget (Utilities|Struct|BreakTargetWrapper Target))) (Variables|Default|GetPlayerToHate))
    (CallFunction|PlayerDied)))

(event Collision|EventActorBeginOverlap
  (params (OtherActor :type Actor%20Object%20Reference)))

(event EventSetHidden
  (params (NewHidden :type Boolean))
  (bind _output_get (Variables|Default|SetHidden NewHidden))
  (if (not _output_get)
    (Animation|PlayAnimMontage "/Game/Characters/NPCs/Demonolgy_follower/Animations/AM_demonologyfollower_combat_taunt.AM_demonologyfollower_combat_taunt" 1.0 "None")))

(event EventTick
  (params (DeltaSeconds :type Float%20%28single-precision%29))
  (|CallParentFunction DeltaSeconds))

(event EventBeginPlay
  (|CallParentFunction)
  (Variables|Default|GetSummonerUID
    (:then
      (if (and (Networking|IsServer) (not (Variables|Default|GetIsThrallVersion)))
        (bind _returnvalue (Class|FuncomGenericLibrary|GetCharacterfromUniqueId (Variables|Default|GetSummonerUID)))
        (CallFunction|AddPlayerHate _returnvalue)))
    (:else)))

(event EventSetSummonerUID
  (params (SummonerUID :type Unique%20ID%20Object%20Reference))
  (Variables|Default|SetSummonerUID SummonerUID)
  (if (and (Networking|IsServer) (not (Variables|Default|GetIsThrallVersion)))
    (bind _returnvalue (Class|FuncomGenericLibrary|GetCharacterfromUniqueId (Variables|Default|GetSummonerUID)))
    (CallFunction|AddPlayerHate _returnvalue)))

(fn ConstructionScript
  (bind _p_demon_effect (Variables|Components|GetP_Demon_Effect))
  (|CallParentFunction)
  (Effects|Components|ParticleSystem|SetActorParameter _p_demon_effect "BoneSocketActor" (Components|GetOwner (Variables|Character|GetMesh)))
  (Transformation|SetAbsolute _p_demon_effect false true false))

(fn OnRepHidden
  (bind _floatingname (Variables|Default|GetFloatingName))
  (bind _mesh (Variables|Character|GetMesh))
  (if (Variables|Default|GetHidden)
    (Rendering|SetVisibility _mesh false false)
    (Development|SetHiddeninGame _floatingname true false)
    (else
      (Rendering|SetVisibility _mesh true false)
      (Development|SetHiddeninGame _floatingname false false))))

(fn BindHateEvents
  (EventDispatchers|BindEventtoSignalonKilled (Variables|Default|GetPlayerToHate) (EventDispatchers|CreateEvent :!event Custom|PlayerDied))
  (EventDispatchers|BindEventtoOnTargetLost (Variables|Default|GetBPTargetDistributionComponent) (EventDispatchers|CreateEvent :!event Custom|TargetLost)))

(fn GetEventLogDeathReason
  (return ""))