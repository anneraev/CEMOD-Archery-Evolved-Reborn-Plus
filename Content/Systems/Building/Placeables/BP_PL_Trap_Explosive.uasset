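; Placeable explosive trap whose activation stops the fuse effects, hides the mesh and plays explosion sound, particles and camera shake.
; It chains async radial damage calls for light wide damage, knock-up, heavy armor-ignoring falloff damage and a close-range cripple.
; Resource actors are gathered into the ignore list to avoid fracturing their destructible meshes.
; Damage is credited to the placement instigator, and the trap reports itself as player damage under its owner's ID.
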(event EventBeginPlay
  (|CallParentFunction))

(event EventPlayTrapActivateEffects
  (bind _returnvalue (CallFunction|GetInstigatorOfPlacement))
  (bind _returnvalue_2 (Transformation|GetActorLocation))
  (bind _self self)
  (bind _staticmesh (Variables|Default|GetStaticMesh))
  (bind _returnvalue_3 (Transformation|GetWorldLocation _staticmesh))
  ;[1 0.6413 0.1882] Effects
  (if (not (Networking|IsDedicatedServer))
    ;;[0.02499 0.09524 0.16] Disable dud effects.
    (bind _fusesound (Variables|Default|GetFuseSound)
      (:then
        (Class|ConanAudioComponent|Stop _fusesound))
      (:else
        _))
    (bind _fusedudsmoke (Variables|Default|GetFuseDudSmoke)
      (:then
        (Components|Activation|Deactivate _fusedudsmoke)
        ;;[0 0.605 0.605] Play Explosion Sound
        (Audio|PlaySoundatLocation (Variables|Default|GetS_Trigger_Activate) _returnvalue_3)
        (Components|Activation|Activate (Variables|Default|GetExplosion) false)
        (Camera|PlayWorldCameraShake "/Game/Items/Explosives/CameraShake_Explosion.CameraShake_Explosion_C" _returnvalue_3 0.0 3072.0 1.0 true)
        (Rendering|SetVisibility _staticmesh false false)
        ;[1 1 1] Do not damage Resource actors, otherwise explosion could cause a fracturation of their destructible meshes
        (if (Networking|IsDedicatedServer)
          (Utilities|Array|Clear (Variables|Default|GetIgnoreActors))
          (else
            (bind _outactors (Actor|GetAllActorsOfClass "/Game/Systems/Survival/Gathering/BP_ResourceActor.BP_ResourceActor_C"))
            (bind _output_get (Variables|Default|SetIgnoreActors _outactors))))
        (Utilities|Array|Add _output_get self)
        (|ApplyRadialDamagewithFalloffAsync 5.0 5.0 _returnvalue_2 8e+02 1024.0 0.0 "/Game/Systems/Progression/DmgTypeHealth_IgnoreArmor_BP.DmgTypeHealth_IgnoreArmor_BP_C" (Variables|Default|GetIgnoreActors) _self _returnvalue "ECC_GameTraceChannel17"
          (:then
            (|ApplyRadialDamageAsync 1.0 _returnvalue_2 9e+02 "/Game/Systems/Combat/DamageTypes/BP_Knockback_KnockUp_CorruptionPerk_Blast.BP_Knockback_KnockUp_CorruptionPerk_Blast_C" (Variables|Default|GetIgnoreActors) _self _returnvalue true "ECC_Visibility"
              (:then
                (|ApplyRadialDamagewithFalloffAsync 5e+02 1e+02 _returnvalue_2 192.0 7.2e+02 2.0 "/Game/Systems/Progression/DmgTypeHealth_IgnoreArmor_BP.DmgTypeHealth_IgnoreArmor_BP_C" (Variables|Default|GetIgnoreActors) _self _returnvalue "ECC_Visibility"
                  (:then
                    (|ApplyRadialDamageAsync 1.0 _returnvalue_2 2.4e+02 "/Game/Systems/Combat/DamageTypes/BP_ProcCrippled.BP_ProcCrippled_C" (Variables|Default|GetIgnoreActors) _self _returnvalue false "ECC_Visibility"))))))))
      (:else))))

(fn ConstructionScript
  (|CallParentFunction))

(fn GetAttackerUniqueID
  (return (Variables|Default|GetOwnerUniqueID)))

(fn IsPlayerDamage
  (return true))

(fn IsThrallDamage
  (return false))