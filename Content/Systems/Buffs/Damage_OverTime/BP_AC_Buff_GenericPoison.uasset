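; BP_AC_Buff_GenericPoison is a damage-over-time poison buff component for a character.
; On each buff tick, it records the buff's cause of death on the owning character through the combat interface.
; It then deals armor-ignoring health damage, scaling per-tick damage by the stack size raised to a configurable exponent.
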(event EventGameplayEffecttoApplyonBuffTick
  (bind _asis_base_bpcombat_interface (Utilities|Casting|CastToIsBaseBPCombatInterface (Variables|Default|GetOwningCharacter)))
  (Default|SetCauseOfDeath _asis_base_bpcombat_interface (Variables|Default|GetCauseOfDeathFromBuff))
  (CallFunction|BuffApplyDamage (* (Variables|Default|GetDamagePerBuffTick) (Math|Float|Power (Math|Conversions|ToFloat(Integer) (Variables|Default|GetStackSize)) (Variables|Default|GetDamageStackExp))) "/Game/Systems/Progression/DmgTypeHealth_IgnoreArmor_BP.DmgTypeHealth_IgnoreArmor_BP_C"))