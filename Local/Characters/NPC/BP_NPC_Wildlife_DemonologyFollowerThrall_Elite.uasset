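; Elite demonology follower thrall with a limited lifespan that turns into a replacement non-thrall NPC when deleted.
; Kills by it, or by the player it follows, extend the lifespan by victim max health, capped at the starting value, and can level it up.
; Deletion triggers transition FX and an emote, then async-spawns the replacement.
; Once AI LOD resumes, the replacement inherits health and summoner ID before the thrall is removed.
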(event Custom|OnResumed
  (params (EventType :type EAILODEventType%20Enum))
  ;[0.09891 0 1] Swap with hostile NPC when lifespan is expired
  (if (Utilities|Enum|Equal(Enum) EventType "Resumed")
    (bind _asconan_character (Utilities|Casting|CastToConanCharacter (Variables|Default|GetSpawnedNPC)))
    (Variables|/Script/Engine.SkeletalMeshComponent|SetAnimationData (Variables|/Script/Engine.Character|GetMesh _asconan_character) (Variables|/Script/Engine.SkeletalMeshComponent|GetAnimationData (Variables|Character|GetMesh)))
    (Class|ConanCharacter|SetIntStat _asconan_character "HealthMax" (Class|ConanCharacter|GetIntStat "HealthMax" "Full"))
    (Class|ConanCharacter|SetIntStat _asconan_character "HealthCurrent" (Class|ConanCharacter|GetIntStat "HealthCurrent" "Full"))
    (Class|BPIDemonFollowerInterface|SetSummonerUID(Message) _asconan_character (Variables|/Script/ConanSandbox.ThrallComponent|GetOwnerUniqueID (Class|ConanCharacter|GetThrallComponent)))
    (Utilities|IsValid (Variables|Default|GetDeleter)
      (:Is%20Valid
        _)
      (:Is%20Not%20Valid
        (Variables|Default|SetDeleter self)
        (Variables|Default|SetDeleterNameInput "Lifetime expired")))
    (|CallParentFunction (Variables|Default|GetDeleterNameInput) (Variables|Default|GetDeleter))))

(event Custom|KilledSomething
  (params (XPReciver :type Actor%20Object%20Reference) (XPGiver :type Actor%20Object%20Reference) (FractionToRecieve :type Float%20%28single-precision%29))
  (bind _returnvalue (Class|ConanCharacter|GetIntStat "Level" "Full"))
  ;[0.09891 0 1] Extend Lifespan When Player or Thrall Gets a kill
  (bind _asconan_character (Utilities|Casting|CastToConanCharacter XPGiver))
  (if (and (< _returnvalue 20) (> (Class|ConanCharacter|GetIntStat _asconan_character "HealthMax" "Full") 75))
    (Class|NPCProgressionSystem|LevelUpto (Class|ConanCharacter|GetNPCProgressionSystem) (+ _returnvalue 1)))
  (CallFunction|SetNewLifespan (Math|Float|Clamp(Float) (+ (* (Variables|Lifespan|GetBaseLifespanAddedPerKill) (Math|Float|Clamp(Float) (Math|Float|NormalizetoRange (Math|Conversions|ToFloat(Integer) (Class|ConanCharacter|GetIntStat _asconan_character "HealthMax" "Full")) 0.0 8e+02) 0.0 2.0)) (Class|ThrallComponent|GetRemainingLifespan (Class|ConanCharacter|GetThrallComponent))) 0.0 (Variables|Lifespan|GetStartingLifespan))))

(event Custom|Multicast_SpawnTransitionFX
  (bind _returnvalue (Transformation|GetActorLocation))
  ;[0.09891 0 1] Swap with hostile NPC when lifespan is expired
  (if (not (Networking|IsDedicatedServer))
    (Effects|SpawnEmitteratLocation "/Game/Sorcery/Rituals/DemonFollower/Effects/P_DemonologyFollower_Transition.P_DemonologyFollower_Transition" (Math|Vector|MakeVector (.x _returnvalue) (.y _returnvalue) (- (.z _returnvalue) 1e+02)))))

(event Custom|BindXPEvent
  (params (UpdatedThrall :type Conan%20Character%20Object%20Reference) (Player :type Conan%20Character%20Object%20Reference))
  (CallFunction|BindOwnerXPEvent true Player))

(event Custom|UnbindXPEvent
  (params (UpdatedThrall :type Conan%20Character%20Object%20Reference) (Player :type Conan%20Character%20Object%20Reference))
  (CallFunction|BindOwnerXPEvent false Player))

(event Custom|BindOwnerXPEvent
  (params (Bind :type Boolean) (Owner :type Conan%20Character%20Object%20Reference))
  (bind _asbase_bpcombat (Utilities|Casting|CastToBaseBPCombat Owner))
  ;[0.09891 0 1] Extend Lifespan When Player or Thrall Gets a kill
  (if Bind
    (EventDispatchers|BindEventtoSignalGiveKillXP _asbase_bpcombat (delegate Custom|KilledSomething))
    (else
      (EventDispatchers|UnbindEventfromSignalGiveKillXP _asbase_bpcombat (delegate Custom|KilledSomething)))))

(event EventBeginPlay
  (|CallParentFunction))

(event Collision|EventActorBeginOverlap
  (params (OtherActor :type Actor%20Object%20Reference)))

(event EventTick
  (params (DeltaSeconds :type Float%20%28single-precision%29))
  (|CallParentFunction DeltaSeconds))

(event EventDeleteThrall
  (params (deleterNameInput :type Text%20%28by%20ref%29) (deleter :type Conan%20Character%20Object%20Reference))
  ;[0.09891 0 1] Swap with hostile NPC when lifespan is expired
  (Variables|Default|SetDeleterNameInput deleterNameInput)
  (Variables|Default|SetDeleter deleter)
  (CallFunction|Vaporize))

(event EventClientAddedThrallComponent
  (|CallParentFunction)
  (if (Networking|IsServer)
    (EventDispatchers|BindEventtoOnThrallStartedFollowingPlayer (Class|ConanCharacter|GetThrallComponent) (delegate Custom|BindXPEvent))
    (EventDispatchers|BindEventtoOnThrallStoppedFollowingPlayer (Class|ConanCharacter|GetThrallComponent) (delegate Custom|UnbindXPEvent))
    (Class|ThrallComponent|InitializeThrallLifespan (Class|ConanCharacter|GetThrallComponent) (Variables|Lifespan|GetStartingLifespan))))

(event EventGiveOwnerKillXP
  (params (XPReciver :type Actor%20Object%20Reference) (XPGiver :type Actor%20Object%20Reference) (FractionToRecieve :type Float%20%28single-precision%29))
  ;[0.09891 0 1] Extend Lifespan When Player or Thrall Gets a kill
  (|CallParentFunction XPReciver XPGiver FractionToRecieve)
  (CallFunction|KilledSomething XPReciver XPGiver FractionToRecieve))

(event EventVaporize
  ;[0.09891 0 1] Swap with hostile NPC when lifespan is expired
  (Class|ThrallSystemComponent|ServerSetFollowing (Class|ConanCharacter|GetThrallSystemComponent (Class|ThrallComponent|GetInteractingPlayer (Class|ConanCharacter|GetThrallComponent))) (Class|ConanCharacter|GetThrallComponent) false)
  (CallFunction|AddTargetLockImmuneReason "vaporize")
  (Collision|SetCollisionEnabled (Variables|Default|GetCapsuleComponent) "NoCollision")
  (CallFunction|MulticastActionEnd) ; Whatever we are currently doing - stop doing it
  (CallFunction|MulticastSpawnTransitionFX)
  (|PlayEmote self "Taunt" false false false false false -1.0
    (:OnEmoteFinished
      (bind (_spawnedpawn _targetlayout _npcbehaviorparameters) (|AsyncSpawnNPC (Variables|Default|GetNonThrallReplacement_SpawnTableID) (Transformation|GetActorTransform) false false)
        (:SpawnSucceeded
          (bind _npc (CallFunction|FinishAsyncTrySpawnNPCfromSpawnTableLowLevel (Variables|Default|GetNonThrallReplacement_SpawnTableID) (Transformation|GetActorLocation) 0.0 0 0 _spawnedpawn _targetlayout _npcbehaviorparameters "WildlifeNPC" 0 false))
          (bind _output_get (Variables|Default|SetSpawnedNPC _npc))
          (EventDispatchers|BindEventtoEventAILOD (Actor|GetComponentbyClass _output_get "/Script/ConanSandbox.AILODComponent") (delegate Custom|OnResumed)))))))

(fn ConstructionScript
  (|CallParentFunction))

(fn SetNewLifespan
  (params (NewLifespan :type Float%20%28single-precision%29))
  (bind _returnvalue (Class|ConanCharacter|GetThrallComponent))
  (Class|ThrallComponent|CancelThrallLifespan _returnvalue)
  (Class|ThrallComponent|InitializeThrallLifespan _returnvalue NewLifespan))