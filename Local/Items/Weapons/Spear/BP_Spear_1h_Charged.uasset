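; One-handed charged spear weapon Blueprint that animates its skeletal mesh from the owner's combat signals, using bow string animations.
; BeginPlay caches third-person state and the anim instance, then binds draw, loop, settle and execute signals, with execute filtered by source.
; Third-person and first-person branches play identical animations.
; Client-side projectile loading from the ammunition item table is unreachable, though EndPlay still calls DestroyLoadedProjectile.
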(event Custom|SignalBowSecondaryLoop
  (if (Variables|Default|GetIn%20Third%20Person)
    (Components|Animation|PlayAnimation (Variables|Default|GetWeaponSkeletalMesh) "/Game/Items/Weapons/Bow/Animations/A_combat_bow_string_heavy_loop.A_combat_bow_string_heavy_loop" false)
    (else
      (Components|Animation|PlayAnimation (Variables|Default|GetWeaponSkeletalMesh) "/Game/Items/Weapons/Bow/Animations/A_combat_bow_string_heavy_loop.A_combat_bow_string_heavy_loop" false))))

(event Custom|SignalBowSecondarySettle
  ;[1 1 1] Basic String Settle
  (if (Variables|Default|GetIn%20Third%20Person)
    (Components|Animation|PlayAnimation (Variables|Default|GetWeaponSkeletalMesh) "/Game/Items/Weapons/Bow/Animations/A_bow_3rd_secondary_special_settle.A_bow_3rd_secondary_special_settle" false)
    (else
      (Components|Animation|PlayAnimation (Variables|Default|GetWeaponSkeletalMesh) "/Game/Items/Weapons/Bow/Animations/A_bow_3rd_secondary_special_settle.A_bow_3rd_secondary_special_settle" false))))

(event Custom|SignalExecute
  (params (Source :type E_AttackSource%20Enum))
  ;[1 1 1] Basic String Execute
  (if (Utilities|Enum|Equal(Enum) Source "NewEnumerator4")
    (if (Variables|Default|GetIn%20Third%20Person)
      (Components|Animation|PlayAnimation (Variables|Default|GetWeaponSkeletalMesh) "/Game/Items/Weapons/Bow/Animations/A_combat_bow_string_heavy_fire.A_combat_bow_string_heavy_fire" false)
      (else
        (Components|Animation|PlayAnimation (Variables|Default|GetWeaponSkeletalMesh) "/Game/Items/Weapons/Bow/Animations/A_combat_bow_string_heavy_fire.A_combat_bow_string_heavy_fire" false)))))

(event Custom|SignalBowSecondaryDraw
  ;[1 1 1] Basic String Draw
  (if (Variables|Default|GetIn%20Third%20Person)
    (Components|Animation|PlayAnimation (Variables|Default|GetWeaponSkeletalMesh) "/Game/Items/Weapons/Bow/Animations/A_combat_bow_string_heavy_charge.A_combat_bow_string_heavy_charge" false)
    (else
      (Components|Animation|PlayAnimation (Variables|Default|GetWeaponSkeletalMesh) "/Game/Items/Weapons/Bow/Animations/A_combat_bow_string_heavy_charge.A_combat_bow_string_heavy_charge" false))))

(event Custom|SignalBowPrimaryDraw
  ;[1 1 1] Basic String Draw
  (if (Variables|Default|GetIn%20Third%20Person)
    (Components|Animation|PlayAnimation (Variables|Default|GetWeaponSkeletalMesh) "/Game/Items/Weapons/Bow/Animations/A_bow_3rd_draw_c2.A_bow_3rd_draw_c2" false)
    (else
      (Components|Animation|PlayAnimation (Variables|Default|GetWeaponSkeletalMesh) "/Game/Items/Weapons/Bow/Animations/A_bow_3rd_draw_c2.A_bow_3rd_draw_c2" false))))

(event EventBeginPlay
  (|CallParentFunction)
  (Utilities|FlowControl|Sequence
    (:then_0
      (Utilities|FlowControl|Sequence
        (:then_0
          (bind _asis_in_third_person_interface (Utilities|Casting|CastToIsInThirdPersonInterface (Components|GetOwner)))
          (bind _returnvalue (Class|IsinThirdPersonInterface|GetIsinThirdPerson _asis_in_third_person_interface))
          (Variables|Default|SetIn%20Third%20Person _returnvalue))
        (:then_1
          (bind _asab_human_male (Utilities|Casting|CastToAB_human_male (Components|SkeletalMesh|GetAnimInstance (Variables|/Script/Engine.Character|GetMesh (CallFunction|GetCharacterOwner)))))
          (Variables|Default|SetAnim%20BP _asab_human_male))))
    (:then_1
      ;[1 1 1] Basic String Draw
      (EventDispatchers|BindEventtoSignalPrimaryStringDraw (.AsBase%20BPCombat (Utilities|Casting|CastToBaseBPCombat (CallFunction|GetCharacterOwner))) (delegate Custom|SignalBowPrimaryDraw)))
    (:then_2
      ;[1 1 1] Basic String Draw
      (EventDispatchers|BindEventtoSignalSecondaryStringDraw (.AsBase%20BPCombat (Utilities|Casting|CastToBaseBPCombat (CallFunction|GetCharacterOwner))) (delegate Custom|SignalBowSecondaryDraw))
      (EventDispatchers|BindEventtoSignalSecondaryStringLoop (.AsBase%20BPCombat (Utilities|Casting|CastToBaseBPCombat (CallFunction|GetCharacterOwner))) (delegate Custom|SignalBowSecondaryLoop))
      ;[1 1 1] Basic String Execute
      (EventDispatchers|AssignSignalBowStringExecute (.AsBase%20BPCombat (Utilities|Casting|CastToBaseBPCombat (CallFunction|GetCharacterOwner))) (delegate Custom|SignalExecute))
      ;[1 1 1] Basic String Settle
      (EventDispatchers|BindEventtoSignalSecondaryStringSettle (.AsBase%20BPCombat (Utilities|Casting|CastToBaseBPCombat (CallFunction|GetCharacterOwner))) (delegate Custom|SignalBowSecondarySettle)))))

(event EventEndPlay
  (params (EndPlayReason :type EEndPlayReason%20Enum :default "Destroyed"))
  (CallFunction|DestroyLoadedProjectile))

(fn ConstructionScript
  (|CallParentFunction))