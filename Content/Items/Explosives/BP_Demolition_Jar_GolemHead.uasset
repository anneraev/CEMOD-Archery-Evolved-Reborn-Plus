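; Golem head variant of the demolition jar, a thrown explosive that rolls with a lit fuse and explodes after about five seconds.
; If PVP is allowed or an attacker UID exists, chained async radial calls apply health, armor-ignoring, knockdown, cripple and explosive damage.
; Non-dedicated instances exclude resource actors to avoid fracturing their meshes.
; It always spawns a large oil fire, multicasts destructible, sound and shake effects, then destroys itself later.
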(event Custom|MulticastExplosionFX
  (bind _returnvalue (Math|Random|RandomFloatinRange 0.75 3.0))
  (bind _destructible (Variables|Default|GetDestructible))
  (bind _staticmesh (Variables|Default|GetStaticMesh))
  (bind _staticmesh_2 (Variables|Default|GetStaticMesh))
  (bind _returnvalue_2 (Transformation|GetWorldLocation _staticmesh_2))
  ;[1 1 1] Explosion
  (Rendering|SetVisibility (Variables|Default|GetStaticMesh) false false)
  (Utilities|FlowControl|Sequence
    (:then_0
      (Collision|SetCollisionEnabled _staticmesh "NoCollision")
      (Physics|SetSimulatePhysics _staticmesh false)
      (Collision|SetCollisionEnabled _destructible "NoCollision")
      (Physics|SetSimulatePhysics _destructible false))
    (:then_1
      (Rendering|SetVisibility (Variables|Default|GetDestructible) true false)
      (Class|DreamworldBlueprints|PlaySoundatLocation "/Game/Sound/SFX/Explosions/explosion_large_debris_Cue.explosion_large_debris_Cue" _returnvalue_2)
      (Camera|PlayWorldCameraShake "/Game/Items/Explosives/CameraShake_Explosion.CameraShake_Explosion_C" _returnvalue_2 0.0 3072.0 1.0 true)
      (Class|DestructibleComponent|ApplyRadiusDamage (Variables|Default|GetDestructible) 5e+04 (Transformation|GetWorldLocation (Variables|Default|GetExplosion)) 15.0 (Math|Random|RandomFloatinRange 1.5e+04 2.25e+04) false)
      (Transformation|SetWorldScale3D (Variables|Default|GetExplosion) (Math|Vector|MakeVector _returnvalue _returnvalue _returnvalue))
      (Transformation|SetWorldRotation (Variables|Default|GetFirelinger) "0,0.000000, 0" false false)
      (Components|Activation|Activate (Variables|Default|GetOilBurst) false)
      (Utilities|FlowControl|Delay 0.5))
    (:then_2
      (Collision|SetActorEnableCollision false))))

(event Custom|MulticastFuse
  (bind _fusesound (Variables|Default|GetFuseSound))
  ;[0 0.605 0.605] Play Fuse Sound
  (Utilities|IsValid _fusesound
    (:Is%20Valid
      (Class|ConanAudioComponent|Play _fusesound 0.0))))

(event Custom|Fuse
  (params (ImpactPoint :type Vector))
  (bind _self self)
  (bind _owningcontroller (Variables|Default|GetOwningController))
  (bind _explosionorigin (Variables|Default|GetExplosionOrigin))
  (bind _returnvalue (Transformation|GetWorldLocation _explosionorigin))
  ;[1 1 1] Fuse Started
  (CallFunction|MulticastFuse)
  (CallFunction|StartRolling ImpactPoint (Variables|Default|GetSpawner))
  (Utilities|FlowControl|Delay 5.0)
  (Utilities|FlowControl|DoOnce false
    (:Completed
      (Utilities|FlowControl|Delay (Math|Random|RandomFloatinRange 0.2 0.5))
      (CallFunction|StopRolling)
      (bind _asconan_game_state (Utilities|Casting|CastToConanGameState (Game|GetGameState)))
      (if (or (Class|ConanGameState|IsPVPAllowed _asconan_game_state) (Utilities|IsValid (Variables|Default|GetAttackerUID)))
        ;[1 1 1] Do not damage Resource actors, otherwise explosion could cause a fracturation of their destructible meshes
        (if (Networking|IsDedicatedServer)
          (Utilities|Array|Clear (Variables|Default|GetIgnoreActors))
          (else
            (bind _outactors (Actor|GetAllActorsOfClass "/Game/Systems/Survival/Gathering/BP_ResourceActor.BP_ResourceActor_C"))
            (bind _output_get (Variables|Default|SetIgnoreActors _outactors))))
        (Utilities|Array|Add _output_get self)
        (|ApplyRadialDamagewithFalloffAsync 5.0 5.0 _returnvalue 8e+02 1024.0 0.0 "/Game/Systems/Progression/DmgTypeHealth_BP.DmgTypeHealth_BP_C" (Variables|Default|GetIgnoreActors) self (Variables|Default|GetOwningController) "ECC_GameTraceChannel17"
          (:then
            (|ApplyRadialDamagewithFalloffAsync 4e+02 1e+02 _returnvalue 8e+02 1024.0 2.0 "/Game/Systems/Progression/DmgTypeHealth_IgnoreArmor_BP.DmgTypeHealth_IgnoreArmor_BP_C" (Variables|Default|GetIgnoreActors) self (Variables|Default|GetOwningController) "ECC_Visibility"
              (:then
                (|ApplyRadialDamageAsync 1.0 _returnvalue 9.3e+02 "/Game/Systems/Combat/DamageTypes/BP_Knockback_Knockdown.BP_Knockback_Knockdown_C" (Variables|Default|GetIgnoreActors) _self _owningcontroller false "ECC_Visibility"
                  (:then
                    (|ApplyRadialDamageAsync 1.0 _returnvalue 1.24e+03 "/Game/Systems/Combat/DamageTypes/BP_ProcCrippled.BP_ProcCrippled_C" (Variables|Default|GetIgnoreActors) _self _owningcontroller false "ECC_Visibility"
                      (:then
                        (|ApplyRadialDamageAsync 1.0 _returnvalue 6.2e+02 "/Game/Systems/Combat/DamageTypes/BP_ProcCrippled.BP_ProcCrippled_C" (Variables|Default|GetIgnoreActors) _self _owningcontroller false "ECC_Visibility"
                          (:then
                            (|ApplyRadialDamagewithFalloffAsync 6e+03 0.0 _returnvalue 8e+02 1024.0 2.0 "/Game/Systems/Combat/Dmg_Explosive.Dmg_Explosive_C" (Variables|Default|GetIgnoreActors) self (Variables|Default|GetOwningController) "ECC_Visibility"
                              (:then
                                _)))))))))))))
      (bind _returnvalue_2 (Game|SpawnActorfromClass "/Game/Items/Explosives/BP_Oil_Fire_Large.BP_Oil_Fire_Large_C" (Math|Transform|MakeTransform (.location (Transformation|GetWorldTransform (Variables|Default|GetOilBurst))) "0, 0, 0" "1,1,1") "AlwaysSpawn" self (Pawn|GetControlledPawn (Variables|Default|GetOwningController))))
      (Variables|/Game/Items/Weapons/Orbs/BP_Orb_Effect_Master.BP_Orb_Effect_Master_C|SetShouldBePlayerDamage _returnvalue_2 true)
      (CallFunction|MulticastExplosionFX)
      (Utilities|FlowControl|Delay 3e+01)
      (Actor|DestroyActor))))

(event Custom|StartRolling
  (params (ImpactPoint :type Vector) (IgnoreActor :type Actor%20Object%20Reference))
  ;[1 1 1] Rolling
  (Collision|IgnoreActorwhenMoving (Variables|Default|GetStaticMesh) IgnoreActor true)
  (Physics|SetSimulatePhysics (Variables|Default|GetStaticMesh) true)
  (Collision|SetCollisionEnabled (Variables|Default|GetStaticMesh) "QueryAndPhysics")
  (if (not (Networking|IsDedicatedServer))
    (Rendering|Components|Light|SetIntensity (Variables|Default|GetFuseLight) 4.5e+02)
    (Components|Activation|Activate (Variables|Default|GetFuseFlame) false)))

(event Custom|StopRolling
  ;[1 1 1] Rolling
  (if (not (Networking|IsDedicatedServer))
    (Physics|SetSimulatePhysics (Variables|Default|GetStaticMesh) false)
    (Collision|SetCollisionEnabled (Variables|Default|GetStaticMesh) "QueryOnly")
    (Rendering|Components|Light|SetIntensity (Variables|Default|GetFuseLight) 4.5e+02)
    (Components|Activation|Deactivate (Variables|Default|GetFuseSmoke))))

(fn ConstructionScript)

(fn GetAttackerUniqueID
  (return (Variables|Default|GetAttackerUID)))

(fn GetImpactRadius
  (return 2.5e+03))

(fn GetImpactStrength
  (return 1.2))

(fn IsPlayerDamage
  ;[1 1 1] Explosive jars are always player damage
  (return true))

(fn IsThrallDamage
  (return false))