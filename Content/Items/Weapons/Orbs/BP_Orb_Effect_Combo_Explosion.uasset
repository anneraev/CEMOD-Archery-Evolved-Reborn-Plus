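; BP_Orb_Effect_Combo_Explosion is an orb weapon combo effect that sets off an explosion at its location on BeginPlay.
; On the server, it chains async radial damage calls credited to the Instigator's controller, each starting from the previous one's "then" output.
; They apply random armor-ignoring damage, knockdown, two crippling procs of different radii and heavy explosive damage.
; The explosion sound plays at the end of this server-only chain.
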(event EventBeginPlay
  (bind _returnvalue (Transformation|GetActorLocation))
  (bind _self self)
  (bind _instigator (Variables|Default|GetInstigator))
  (bind _returnvalue_2 (Pawn|GetController _instigator))
  (|CallParentFunction)
  (if (Networking|IsServer)
    (|ApplyRadialDamageAsync (Math|Random|RandomFloatinRange 5e+01 2e+02) _returnvalue 1024.0 "/Game/Systems/Progression/DmgTypeHealth_IgnoreArmor_BP.DmgTypeHealth_IgnoreArmor_BP_C" 0 _self _returnvalue_2 false "ECC_Visibility"
      (:then
        (|ApplyRadialDamageAsync 1.0 _returnvalue 1.28e+03 "/Game/Systems/Combat/DamageTypes/BP_Knockback_Knockdown.BP_Knockback_Knockdown_C" 0 _self _returnvalue_2 false "ECC_Visibility"
          (:then
            (|ApplyRadialDamageAsync 1.0 _returnvalue 1.28e+03 "/Game/Systems/Combat/DamageTypes/BP_ProcCrippled.BP_ProcCrippled_C" 0 _self _returnvalue_2 false "ECC_Visibility"
              (:then
                (|ApplyRadialDamageAsync 1.0 _returnvalue 6.4e+02 "/Game/Systems/Combat/DamageTypes/BP_ProcCrippled.BP_ProcCrippled_C" 0 0 _returnvalue_2 false "ECC_Visibility"
                  (:then
                    (|ApplyRadialDamageAsync 2.5e+03 _returnvalue 1024.0 "/Game/Systems/Combat/Dmg_Explosive.Dmg_Explosive_C" 0 _self _returnvalue_2 false "ECC_Visibility"
                      (:then
                        (Class|DreamworldBlueprints|PlaySoundatLocation (Variables|Default|GetExplosion_Sound) _returnvalue)))))))))))))

(fn ConstructionScript
  (|CallParentFunction))