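; Orb weapon effect that leaves a ground fire, dealing repeated area damage around its location.
; On BeginPlay it sets HasExploded, and the server starts a looping timer that applies two async radial hits within the sphere's radius: armor-ignoring health damage, then explosive damage scaled inversely by the fade delay.
; Non-server instances handle particle collision logic, triggered through the HasExploded RepNotify.
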(event Custom|DoDamage
  (bind _returnvalue (Transformation|GetActorLocation))
  (bind _returnvalue_2 (Game|GetInstigatorController))
  (bind _self self)
  (bind _sphere (Variables|Default|GetSphere))
  (bind _sphereradius (Variables|/Script/Engine.SphereComponent|GetSphereRadius _sphere))
  (|ApplyRadialDamageAsync 8.0 _returnvalue _sphereradius "/Game/Systems/Progression/DmgTypeHealth_IgnoreArmor_BP.DmgTypeHealth_IgnoreArmor_BP_C" 0 _self _returnvalue_2 true "ECC_Visibility"
    (:then
      (|ApplyRadialDamageAsync (/ 1e+03 (Variables|Default|GetDelayUntilFadeEffects)) _returnvalue _sphereradius "/Game/Systems/Combat/Dmg_Explosive.Dmg_Explosive_C" 0 _self _returnvalue_2 true "ECC_Visibility"))))

(event Custom|Orb_Fire_Collide
  (params (EventName :type Name) (EmitterTime :type Float%20%28single-precision%29) (ParticleTime :type Integer) (Location :type Vector) (Velocity :type Vector) (Direction :type Vector) (Normal :type Vector) (BoneName :type Name) (PhysMat :type Physical%20Material%20Object%20Reference))
  (if (not (Networking|IsServer))
    (EventDispatchers|AssignOnParticleCollide (Variables|Default|GetParticleSystem) (delegate Custom|Orb_Fire_Collide))))

(event Custom|ParticleStart
  (if (not (Networking|IsServer))
    (CallFunction|OrbFireCollide "None" 0.0 0 "0, 0, 0" "0, 0, 0" "0, 0, 0" "0, 0, 0" "None")))

(event EventBeginPlay
  (|CallParentFunction)
  (Variables|Default|SetHasExploded true)
  (if (Networking|IsServer)
    (Utilities|Time|SetTimerbyEvent (delegate Custom|DoDamage) 0.5 true)))

(fn ConstructionScript
  (|CallParentFunction))

(fn OnRepHasExploded
  (CallFunction|ParticleStart))