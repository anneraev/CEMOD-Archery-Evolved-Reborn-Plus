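; Base bow launcher item that applies power-charge effects to fired projectiles when SetCombo runs.
; It copies the combatant's current combo onto the projectile, adding on-hit and on-block damage modifiers for each listed damage type while in a specific combat substate.
; In that substate, owners with the Accuracy_40 perk also get a knockback class scaled by charge: flinch, push or knockdown.
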(event EventSetCombo
  (params (BaseCombat :type Base%20BP%20Combat%20Object%20Reference) (BaseProjectile :type BP%20Base%20Projectile%20Object%20Reference))
  (CallFunction|HandlePowerChargeforDamageType BaseCombat BaseProjectile)
  (CallFunction|HandlePowerChargeforPerk BaseCombat BaseProjectile))

(fn HandlePowerChargeforDamageType
  (params (Combat :type Base%20BP%20Combat%20Object%20Reference) (Projectile :type BP%20Base%20Projectile%20Object%20Reference))
  (bind _returnvalue (|GetPowerChargeMod))
  (bind _output_get (LocalVariables|Setlocal%20Combat Combat))
  (bind _combocurrent (Default|GetComboCurrent _output_get))
  (LocalVariables|Setlocal%20Combo _combocurrent)
  (for _array_element (Variables|PowerCharge|GetPowerChargeMultipliers)
    (if (Default|InSubstate (LocalVariables|Getlocal%20Combat) "NewEnumerator25")
      (Utilities|Array|Add (.DamageModifiers (Utilities|Struct|BreakSTR_ComboStep (LocalVariables|Getlocal%20Combo))) (Utilities|Struct|MakeSTR_ComboStepDamageMod _array_element _returnvalue _returnvalue))))
  (Variables|/Game/Items/Weapons/BP_BaseProjectile.BP_BaseProjectile_C|SetComboStructure Projectile (LocalVariables|Getlocal%20Combo))
  (return))

(fn HandlePowerChargeforPerk
  (params (Combat :type Base%20BP%20Combat%20Object%20Reference) (Projectile :type BP%20Base%20Projectile%20Object%20Reference))
  (bind _output_get (LocalVariables|Setlocal%20Combat Combat))
  (Utilities|IsValid _output_get
    (:Is%20Valid
      (bind _output_get_2 (LocalVariables|Setlocal%20Projectile Projectile))
      (Utilities|IsValid _output_get_2
        (:Is%20Valid
          (bind _combocurrent (Default|GetComboCurrent (LocalVariables|Getlocal%20Combat)))
          (LocalVariables|Setlocal%20Combo _combocurrent)
          (if (Default|InSubstate (LocalVariables|Getlocal%20Combat) "NewEnumerator25")
            (bind _asi_perk_system_owner_interface (Utilities|Casting|CastToI_PerkSystemOwnerInterface (LocalVariables|Getlocal%20Combat))
              (:then
                (bind _perksysteminterface (Default|GetPerkSystem _asi_perk_system_owner_interface))
                (bind _hasperk (Default|HasPerk _perksysteminterface "Accuracy_40"))
                (if _hasperk
                  (bind _structout (Utilities|Struct|SetmembersinSTR_ComboStep (Variables|/Game/Items/Weapons/BP_BaseProjectile.BP_BaseProjectile_C|GetComboStructure (LocalVariables|Getlocal%20Projectile)) (Utilities|Select :Index (Math|Float|Floor (Math|Float|MapRangeUnclamped (Default|GetPowerChargeModifier (LocalVariables|Getlocal%20Combat)) 0.0 1.0 0.0 2.0)) :Option%200 "/Game/Systems/Combat/DamageTypes/BP_Knockback_FlinchAway_Accuracy40_Perk.BP_Knockback_FlinchAway_Accuracy40_Perk_C" :Option%201 "/Game/Systems/Combat/DamageTypes/BP_Knockback_PushAway_Accuracy40_Perk.BP_Knockback_PushAway_Accuracy40_Perk_C" :Option%202 "/Game/Systems/Combat/DamageTypes/BP_Knockback_Knockdown_Accuracy40_Perk.BP_Knockback_Knockdown_Accuracy40_Perk_C")))
                  (Variables|/Game/Items/Weapons/BP_BaseProjectile.BP_BaseProjectile_C|SetComboStructure (LocalVariables|Getlocal%20Projectile) _structout)
                  (return)
                  (else
                    (return))))
              (:CastFailed
                _)))
          (return))
        (:Is%20Not%20Valid
          _)))
    (:Is%20Not%20Valid
      _))
  (return))